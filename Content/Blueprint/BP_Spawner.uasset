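; BP_Spawner is an enemy spawner that holds a queue of enemy classes and spawns them at its own transform.
; AddEnemyQueue appends a class, then spawns the front entry immediately if no BP_Enemy overlaps its sphere collision.
; SpawnEnemy removes each spawned entry and reports whether the queue had one.
; A timer set on BeginPlay also calls SpawnEnemy, without the overlap check.
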(event `self.ReceiveBeginPlay`
  (`KismetSystemLibrary.K2_SetTimerDelegate` (delegate `TryToSpawn`) 2.0))

(event `TryToSpawn`
  (`self.SpawnEnemy`))

(fn `AddEnemyQueue`
  (params (EnemyClass :type "/Game/Blueprint/BP_Enemy Class Reference (by ref)"))
  (`KismetArrayLibrary.Array_Add` (`self.EnemyQueue`) EnemyClass)
  (if (not (`KismetArrayLibrary.Array_IsValidIndex` (`PrimitiveComponent.GetOverlappingActors` (`self.SphereColl`) "/Game/Blueprint/BP_Enemy.BP_Enemy_C")))
    (`self.SpawnEnemy`)))

(fn `SpawnEnemy`
  (returns (Succes :type Boolean))
  (if (`KismetArrayLibrary.Array_IsValidIndex` (`self.EnemyQueue`))
    (`|SpawnActorFromClass` (`|GetArrayItem` (`self.EnemyQueue`)) (`self.GetTransform`) "Undefined" "MultiplyWithRoot" null null)
    (`KismetArrayLibrary.Array_Remove` (`self.EnemyQueue`))
    (return true)
    (else
      (return false))))

(fn `UserConstructionScript`)